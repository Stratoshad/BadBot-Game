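; BP_SphereSpawner is an actor that repeatedly spawns BP_SmallSphere actors at random positions around itself.
; BeginPlay starts a looping timer, rolling its interval once between the configured minimum and maximum.
; SpawnSphere uses random rotation and builds location from separate calls to a random-point-in-radius helper, clamping Z with a zero world-height minimum.
; Tick draws a debug sphere showing the spawn radius.
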(event Custom|SpawnSphere
  (bind _randompoint (CallFunction|GetRandomPointinSphereRadius))
  ;[1 0.3923 0.2812] Start Sphere Spawn Timer
  (Game|SpawnActorfromClass "/Game/Blueprints/SmallSphere/BP_SmallSphere.BP_SmallSphere_C" (Math|Transform|MakeTransform (Math|Vector|MakeVector (.x _randompoint) (.y _randompoint) (Math|Float|Clamp(Float) (.z _randompoint) 0.0 (.z _randompoint))) (Math|Random|RandomRotator false) "1.000000,1.000000,1.000000") "Undefined" "MultiplyWithRoot" 0 0))

(event EventBeginPlay
  ;[1 0.3923 0.2812] Start Sphere Spawn Timer
  (Utilities|Time|SetTimerbyEvent (EventDispatchers|CreateEvent :!event Custom|SpawnSphere) (Math|Random|RandomFloatinRange (Variables|SphereSpawner|GetSpawnTimeMin) (Variables|SphereSpawner|GetSpawnTimeMax)) true))

(event EventTick
  (params (DeltaSeconds :type Float%20%28single-precision%29))
  (Rendering|Debug|DrawDebugSphere (Transformation|GetActorLocation) (Variables|SphereSpawner|GetSpawnRadius) 12 "(R=1.000000,G=1.000000,B=1.000000,A=1.000000)" 0.0))

(fn ConstructionScript)

(fn GetRandomPointinSphereRadius
  (return (+ (Transformation|GetActorLocation) (* (Math|Vector|GetForwardVector (Math|Random|RandomRotator false)) (Math|Random|RandomFloatinRange 0.0 (Variables|SphereSpawner|GetSpawnRadius))))))